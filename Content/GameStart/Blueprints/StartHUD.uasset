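; StartHUD is the HUD for the game's start screen, drawing a title image with a clickable Start hit box.
; Art and hit box scale by screen width from a 960x640 layout, offset vertically by a third of the leftover height.
; Clicking Start shows a loading overlay, then calls both LoadStreamLevel and OpenLevel on ThirdPersonExampleMap.
; On BeginPlay it fetches the high score from a Heroku web service into VRPacManGameInstance.
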(event Custom|OnGetResult
  ;[1 1 1] SaveHigeScore
  (bind _asvrpac_man_game_instance (Utilities|Casting|CastToVRPacManGameInstance (Game|GetGameInstance)))
  (Variables|/Game/VRPacManGameInstance.VRPacManGameInstance_C|SetHighScore _asvrpac_man_game_instance (Math|Conversions|ToInteger(Byte) (Class|JsonFieldData|GetString (Variables|Default|GetJsonData) "score"))))

(event EventDrawHUD
  (params (SizeX :type Integer) (SizeY :type Integer))
  ;[1 1 1] Draw HUD
  (Variables|Default|SetScale (/ (Math|Conversions|ToFloat(Integer) SizeX) 9.6e+02))
  (Canvas|DrawTexture "/Game/GameStart/Textures/Top.Top" 0.0 (/ (- (Math|Conversions|ToFloat(Integer) SizeY) (* (Variables|Default|GetScale) 6.4e+02)) 3.0) 9.6e+02 6.4e+02 0.0 0.0 1.0 1.0 "(R=1.000000,G=1.000000,B=1.000000,A=1.000000)" "BLEND_Opaque" (Variables|Default|GetScale))
  (if (Variables|Default|GetisLoading)
    (Canvas|DrawTexture "/Game/GameStart/Textures/Loading.Loading" 0.0 (/ (- (Math|Conversions|ToFloat(Integer) SizeY) (* (Variables|Default|GetScale) 6.4e+02)) 3.0) 9.6e+02 6.4e+02 0.0 0.0 1.0 1.0 "(R=1.000000,G=1.000000,B=1.000000,A=1.000000)" "BLEND_Translucent" (Variables|Default|GetScale))
    (else
      (Class|HUD|AddHitBox (+ (* (Math|Vector2D|MakeVector2D 375.0 3.7e+02) (Variables|Default|GetScale)) (Math|Vector2D|MakeVector2D 0.0 (/ (- (Math|Conversions|ToFloat(Integer) SizeY) (* (Variables|Default|GetScale) 6.4e+02)) 3.0))) (* (Math|Vector2D|MakeVector2D 2.5e+02 58.0) (Variables|Default|GetScale)) "Start" false))))

(event EventHitBoxClick
  (params (BoxName :type Name))
  ;[1 1 1] HitBoxClicked
  (switch name BoxName
    (:Start
      (Variables|Default|SetisLoading true)
      (Game|LoadStreamLevel(byName) "ThirdPersonExampleMap" false)
      (Game|OpenLevel(byName) "ThirdPersonExampleMap"))))

(event EventBeginPlay
  ;[1 1 1] SaveHigeScore
  (Variables|Default|SetJsonData (Class|JsonFieldData|GetRequest "https://supermarche-madame-4325.herokuapp.com/HighScore"))
  (EventDispatchers|BindEventtoOnGetResult (Variables|Default|GetJsonData) (delegate Custom|OnGetResult)))

(fn ConstructionScript)